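; BP_Hexagon is a hexagon tile actor that gets a random look when play begins.
; On BeginPlay it rolls a random integer and switches the hexagon mesh's first material slot to a normal, ice, oil or explosion material.
; Only the material changes; the Blueprint holds no gameplay behavior for these types and its construction script is empty.
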(event `self.ReceiveBeginPlay`
  (bind _hexagonmesh (`self.HexagonMesh`))
  (switch `int` (`KismetMathLibrary.RandomIntegerInRange` 0 3)
    (:`0`
      (`PrimitiveComponent.SetMaterial` _hexagonmesh 0 (`self.NormalMat`)))
    (:`1`
      (`PrimitiveComponent.SetMaterial` _hexagonmesh 0 (`self.IceMat`)))
    (:`2`
      (`PrimitiveComponent.SetMaterial` _hexagonmesh 0 (`self.OilMat`)))
    (:`3`
      (`PrimitiveComponent.SetMaterial` _hexagonmesh 0 (`self.ExplosionMat`)))))

(fn `UserConstructionScript`)