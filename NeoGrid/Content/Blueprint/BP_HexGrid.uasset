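; BP_HexGrid is a grid spawner that lays out a field of BP_Hexagon actors when play begins.
; Nested loops over GridHeight and GridWidth derive each position from HexWidth and HexHeight, with columns along X and rows along Y.
; Odd rows shift along X by a HexHeight-based offset to stagger the hexagons.
; Positions are absolute world coordinates, independent of the grid actor's transform, and the construction script is empty.
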(event `self.ReceiveBeginPlay`
  (for _index (range (`self.GridHeight`))
    (for _index_2 (range (`self.GridWidth`))
      (if (== (mod (`KismetMathLibrary.Conv_IntToDouble` _index) 2.0) 0.0)
        (bind _returnvalue (`KismetMathLibrary.Conv_IntToDouble` (* _index_2 (* (`self.HexWidth`) 0.75))))
        (bind _returnvalue_2 (* _index (`self.HexHeight`)))
        (`|SpawnActorFromClass` "/Game/Blueprint/BP_Hexagon.BP_Hexagon_C" (`KismetMathLibrary.MakeTransform` (`KismetMathLibrary.MakeVector` _returnvalue _returnvalue_2)) "Undefined" "MultiplyWithRoot" null null)
        (else
          (`|SpawnActorFromClass` "/Game/Blueprint/BP_Hexagon.BP_Hexagon_C" (`KismetMathLibrary.MakeTransform` (`KismetMathLibrary.MakeVector` (+ _returnvalue (/ (`self.HexHeight`) 1.73)) _returnvalue_2)) "Undefined" "MultiplyWithRoot" null null))))))

(fn `UserConstructionScript`)