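; Player-controlled red car Blueprint, apparently Character-based, driven through its own Red-specific input bindings for movement and jumping.
; Forward input moves it along the control rotation's yaw, while right input moves it along a fixed world negative-Y axis, independent of facing.
; The jump action starts and stops the built-in jump on press and release.
; An interpolated camera-rotation snippet is left unconnected, and Tick is empty.
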(event `InputAction|JumpRed`
  (params (Key :type "Key Structure"))
  ;[1 1 1] Jump with G
  (:`Pressed`
    (`self.Jump`))
  (:`Released`
    (`self.StopJumping`)))

(event `InputAxis|MoveForwarRed`
  (params (AxisValue :type "Float (single-precision)"))
  (bind (_returnvalue_roll _returnvalue_pitch _returnvalue_yaw) (`KismetMathLibrary.BreakRotator` (`self.GetControlRotation`)))
  ;[1 1 1] Movimiento con W/S
  (`self.AddMovementInput` (`KismetMathLibrary.GetForwardVector` (`KismetMathLibrary.MakeRotator` 0.0 0.0 _returnvalue_yaw)) AxisValue))

(event `InputAxis|MoveRightRed`
  (params (AxisValue :type "Float (single-precision)"))
  (`self.AddMovementInput` (`KismetMathLibrary.MakeVector` 0.0 -1.0) AxisValue))

(event `self.ReceiveTick`
  (params (DeltaSeconds :type "Float (single-precision)")))

(fn `UserConstructionScript`)